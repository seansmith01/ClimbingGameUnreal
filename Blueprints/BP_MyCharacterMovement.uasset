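; Player character Blueprint that adds camera zoom, jump and hover tuning values, and a bubble visual for hovering.
; Zoom inputs step the camera boom length within clamped limits, while BeginPlay sets the jump power and hover fall speed variables.
; Tick syncs Bubble visibility to the Hovering flag and re-applies the Quinn animation Blueprint to the mesh every frame.
; These graphs contain no logic that performs the jump or hover.
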(event `InputAction|ZoomCameraIn`
  (params (Key :type "Key Structure"))
  (:`Pressed`
    (set `SpringArmComponent.TargetArmLength` (`KismetMathLibrary.FClamp` (- (`SpringArmComponent.TargetArmLength` (`self.CameraBoom`)) 50.0) 200.0 2000.0) (`self.CameraBoom`))))

(event `self.ReceiveBeginPlay`
  (set `self.JumpPowerIncreaseRate` 1000.0)
  (set `self.MaxJumpPower` 750.0)
  (set `self.hoveringFallSpeed` -200.0))

(event `InputAction|ZoomCameraOut`
  (params (Key :type "Key Structure"))
  (:`Pressed`
    (set `SpringArmComponent.TargetArmLength` (`KismetMathLibrary.FClamp` (+ (`SpringArmComponent.TargetArmLength` (`self.CameraBoom`)) 50.0) 200.0 2000.0) (`self.CameraBoom`))))

(event `self.ReceiveTick`
  (params (DeltaSeconds :type "Float (single-precision)"))
  (`SceneComponent.SetVisibility` (`self.Bubble`) (`self.hovering`) false)
  (`SkeletalMeshComponent.SetAnimInstanceClass` (`self.Mesh`) "/Game/Characters/Mannequins/Animations/ABP_Quinn.ABP_Quinn_C"))

(fn `UserConstructionScript`)